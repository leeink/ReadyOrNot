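; BP_MainGameMode is the game mode that runs the win and lose conditions and switches between the matching screens.
; BeginPlay caches the BP_LHM_Player character and creates in-game, clear and game-over widgets, showing the in-game one.
; Tick polls for Neutralize reaching a threshold (clear) or player HP running out (game over), with clear taking priority.
; Either outcome swaps the HUD for its end screen and shows the mouse cursor, with no guard against repeat firing.
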(event `self.ReceiveBeginPlay`
  (`|ExecutionSequence`
    (:`then_0`
      (bind _asbp_lhm_player (cast `/Game/LHM/LHM_BP/Player/Blueprints/BP_LHM_Player` (`GameplayStatics.GetPlayerCharacter` 0)))
      (set `self.Character` _asbp_lhm_player))
    (:`then_1`
      (bind _returnvalue (`|CreateWidget` "/Game/LDG/Blueprint/BP_InGameWidget.BP_InGameWidget_C"))
      (bind _output_get (set `self.InGameWidget` _returnvalue))
      (bind _returnvalue_2 (`|CreateWidget` "/Game/LDG/Blueprint/BP_ClearGameWidget.BP_ClearGameWidget_C"))
      (set `self.ClearGameWidget` _returnvalue_2)
      (bind _returnvalue_3 (`|CreateWidget` "/Game/LDG/Blueprint/WBP_GameOverWidget.WBP_GameOverWidget_C"))
      (set `self.GameOverWdiget` _returnvalue_3)
      (`UserWidget.AddToViewport` _output_get 0))))

(event `self.ReceiveTick`
  (params (DeltaSeconds :type "Float (single-precision)"))
  (if (>= (`self.Neutralize`) 10)
    (`self.GameClear`)
    (elif (<= (`/Game/LHM/LHM_BP/Player/Blueprints/BP_LHM_Player.HP` (`self.Character`)) 0.0)
      (`self.GameOver`))))

(event `GameClear`
  (set `PlayerController.bShowMouseCursor` true (`GameplayStatics.GetPlayerController` 0))
  (`Widget.RemoveFromParent` (`self.InGameWidget`))
  (`UserWidget.AddToViewport` (`self.ClearGameWidget`) 0))

(event `GameOver`
  (set `PlayerController.bShowMouseCursor` true (`GameplayStatics.GetPlayerController` 0))
  (`Widget.RemoveFromParent` (`self.InGameWidget`))
  (`UserWidget.AddToViewport` (`self.GameOverWdiget`) 0))

(fn `UserConstructionScript`)