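; Enemy pistol Blueprint that fires a hitscan shot to damage the player.
; Fire plays muzzle flash and sound, then runs a debug-drawn Visibility multi-trace along the actor's right vector.
; Each hit spawns a BP_ProjectileField, and player hits apply BPGunComponent damage.
; BeginPlay caches only the first BP_Enemy and BP_Surrender_Enemy found as trace ignores; Reload is a print stub.
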(event `self.ReceiveBeginPlay`
  (`parent.ReceiveBeginPlay`)
  (bind _returnvalue (`GameplayStatics.GetActorOfClass` "/Game/CHJ/Blueprints/BP_Enemy.BP_Enemy_C"))
  (bind _returnvalue_2 (`GameplayStatics.GetActorOfClass` "/Game/CHJ/Blueprints/BP_Surrender_Enemy.BP_Surrender_Enemy_C"))
  (set `self.IgnoreActors` (`|MakeArray` _returnvalue _returnvalue_2 :!type "/Game/CHJ/Blueprints/BP_EnemyBase Object Reference")))

(event `self.Fire`
  (bind _returnvalue (`self.K2_GetActorLocation`))
  (bind (_returnvalue_location _returnvalue_rotation _returnvalue_scale) (`KismetMathLibrary.BreakTransform` (`SceneComponent.GetSocketTransform` (`self.BP_GunComponent`) "MuzzleFlash" "RTS_World")))
  (`GameplayStatics.SpawnEmitterAtLocation` "/Game/Asset/MilitaryWeapSilver/FX/P_AssaultRifle_MuzzleFlash.P_AssaultRifle_MuzzleFlash" _returnvalue_location _returnvalue_rotation _returnvalue_scale)
  (`GameplayStatics.PlaySoundAtLocation` "/Game/Asset/MilitaryWeapSilver/Sound/Rifle/Wavs/RifleA_Fire03.RifleA_Fire03" _returnvalue (struct) 1.0 1.0 0.0 null null null null)
  (bind _outhits (`KismetSystemLibrary.LineTraceMulti` _returnvalue (+ _returnvalue (* (`self.GetActorRightVector`) 10000.0)) "TraceTypeQuery1" false (`self.IgnoreActors`) "ForDuration" true (struct :`R` 0.073745 :`G` 0.217417 :`B` 0.847222 :`A` 1.0) (struct :`G` 1.0 :`A` 1.0) 2.0))
  (for _array_element _outhits
    (`|ExecutionSequence`
      (:`then_0`
        (bind (_bblockinghit _binitialoverlap _time _distance _location _impactpoint _normal _impactnormal _physmat _hitactor) (`GameplayStatics.BreakHitResult` _array_element))
        (bind _asbp_lhm_player (cast `/Game/LHM/LHM_BP/Player/Blueprints/BP_LHM_Player` _hitactor))
        (`/Game/LHM/LHM_BP/Player/Blueprints/BP_LHM_Player.Damage` _asbp_lhm_player (`/Game/LDG/Blueprint/BP_GunComponent.Damage` (`self.BP_GunComponent`)))
        (`KismetSystemLibrary.PrintString` (`KismetStringLibrary.Conv_DoubleToString` (`/Game/LHM/LHM_BP/Player/Blueprints/BP_LHM_Player.HP` _asbp_lhm_player))))
      (:`then_1`
        (`|SpawnActorFromClass` "/Game/LDG/Blueprint/BP_ProjectileField.BP_ProjectileField_C" (`KismetMathLibrary.MakeTransform` _location) "Undefined" "MultiplyWithRoot" null null)))))

(event `self.Reload`
  (`KismetSystemLibrary.PrintString` "Reload"))

(fn `UserConstructionScript`
  (`parent.UserConstructionScript`))