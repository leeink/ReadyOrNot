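; BP_Ghost is a hitscan gun for BP_LHM_Player, with ammo, reload and a placeholder secondary aim that only prints.
; MainAttack spends a round, plays muzzle flash, sound and camera shake, then multi-line traces from the muzzle along the player camera's forward direction, ignoring the player.
; Each hit damages any enemy through its BP_EnemyFSM component and spawns a BP_ProjectileField at the impact.
; The trace still draws debug lines.
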(event `self.ReceiveBeginPlay`
  (bind _returnvalue (`GameplayStatics.GetActorOfClass` "/Game/LHM/LHM_BP/Player/Blueprints/BP_LHM_Player.BP_LHM_Player_C"))
  (bind _output_get (set `self.Character` _returnvalue))
  (`KismetArrayLibrary.Array_Set` (`self.IgnoreActor`) 0 _output_get))

(event `/Game/LDG/Blueprint/BPI_MainAttackable.MainAttack`
  (bind _ammo (`self.Ammo`))
  (bind _character (`self.Character`))
  (bind _returnvalue (`SceneComponent.GetSocketLocation` (`self.GhostMesh`) "MuzzleFlash"))
  (bind _returnvalue_2 (`self.K2_GetActorLocation` _character))
  (if (> _ammo 0)
    (set `self.Ammo` (- _ammo 1))
    (`GameplayStatics.SpawnEmitterAtLocation` "/Game/Asset/MilitaryWeapSilver/FX/P_AssaultRifle_MuzzleFlash.P_AssaultRifle_MuzzleFlash" _returnvalue)
    (`GameplayStatics.PlaySoundAtLocation` "/Game/Asset/MilitaryWeapSilver/Sound/Pistol/Wavs/PistolA_Fire01.PistolA_Fire01" _returnvalue (struct) 1.0 1.0 0.0 null null null null)
    (`GameplayStatics.PlayWorldCameraShake` "/Game/LHM/LHM_BP/BP_CameraShake.BP_CameraShake_C" _returnvalue_2 100.0 1000.0)
    (bind _outhits (`KismetSystemLibrary.LineTraceMulti` _returnvalue (+ _returnvalue_2 (* (`SceneComponent.GetForwardVector` (`/Game/LHM/LHM_BP/Player/Blueprints/BP_LHM_Player.FirstPersonCamera` _character)) 10000.0)) "TraceTypeQuery1" false (`self.IgnoreActor`) "ForDuration" true (struct :`R` 1.0 :`A` 1.0) (struct :`G` 1.0 :`A` 1.0) 1.0))
    (for _array_element _outhits
      (`|ExecutionSequence`
        (:`then_0`
          (bind (_bblockinghit _binitialoverlap _time _distance _location _impactpoint _normal _impactnormal _physmat _hitactor) (`GameplayStatics.BreakHitResult` _array_element))
          (bind _asbp_enemy_base (cast `/Game/CHJ/Blueprints/BP_EnemyBase` _hitactor))
          (`/Game/CHJ/Blueprints/BP_EnemyFSM.Damage` (`self.GetComponentByClass` _asbp_enemy_base "/Game/CHJ/Blueprints/BP_EnemyFSM.BP_EnemyFSM_C") (`self.Damage`)))
        (:`then_1`
          (`|SpawnActorFromClass` "/Game/LDG/Blueprint/BP_ProjectileField.BP_ProjectileField_C" (`KismetMathLibrary.MakeTransform` _location) "Undefined" "MultiplyWithRoot" null null))))))

(event `/Game/LDG/Blueprint/BPI_SubAttackable.SubAttackable`
  (`KismetSystemLibrary.PrintString` "Ghost Aim"))

(event `/Game/LDG/Blueprint/BPI_Reloadable.Reloadable`
  (set `self.Ammo` (`self.MaxAmmo`)))

(fn `UserConstructionScript`)