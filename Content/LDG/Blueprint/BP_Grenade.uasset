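; BP_Grenade is a thrown grenade that damages the player and enemies.
; MainAttack launches the physics mesh along the player camera's forward vector, then after a fuse delay enables two overlap volumes, plays explosion effects and destroys itself.
; The explosion volume damages players directly and enemies through their BP_EnemyFSM component.
; The camera volume triggers a camera shake and spawns a BP_ProjectileField at any overlapped player.
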(event `self.ReceiveBeginPlay`
  (bind _asbp_lhm_player (cast `/Game/LHM/LHM_BP/Player/Blueprints/BP_LHM_Player` (`GameplayStatics.GetPlayerCharacter` 0)))
  (set `self.Character` _asbp_lhm_player))

(event `/Game/LDG/Blueprint/BPI_MainAttackable.MainAttack`
  (bind _granademesh (`self.GranadeMesh`))
  (bind _returnvalue (`SceneComponent.K2_GetComponentLocation` _granademesh))
  ;[1 1 1] Explosion
  (`PrimitiveComponent.SetSimulatePhysics` _granademesh true)
  (`PrimitiveComponent.SetPhysicsLinearVelocity` _granademesh (* (`SceneComponent.GetForwardVector` (`/Game/LHM/LHM_BP/Player/Blueprints/BP_LHM_Player.FirstPersonCamera` (`self.Character`))) (`self.Speed`)) false "None")
  (`KismetSystemLibrary.Delay` 3.0)
  (`PrimitiveComponent.SetCollisionEnabled` (`self.ExplosionCollision`) "QueryOnly")
  (`PrimitiveComponent.SetCollisionEnabled` (`self.CameraCollsion`) "QueryOnly")
  (`GameplayStatics.PlaySoundAtLocation` "/Game/Asset/MilitaryWeapSilver/Sound/GrenadeLauncher/Wavs/GrenadeLauncher_Explosion01.GrenadeLauncher_Explosion01" _returnvalue (struct) 1.0 1.0 0.0 null null null null)
  (`GameplayStatics.SpawnEmitterAtLocation` "/Game/Asset/MilitaryWeapSilver/FX/P_Grenade_Explosion_01.P_Grenade_Explosion_01" _returnvalue (struct) (3.0 3.0 3.0))
  (`self.K2_DestroyActor`))

(event `self.ExplosionCollision.OnComponentBeginOverlap`
  (params (OverlappedComponent :type "PrimitiveComponent Object Reference") (OtherActor :type "Actor Object Reference") (OtherComp :type "PrimitiveComponent Object Reference") (OtherBodyIndex :type Integer) (bFromSweep :type Boolean) (SweepResult :type "HitResult Structure (by ref)"))
  (bind _damage (`self.Damage`))
  ;[1 1 1] Damage
  (`|ExecutionSequence`
    (:`then_0`
      (bind _asbp_lhm_player (cast `/Game/LHM/LHM_BP/Player/Blueprints/BP_LHM_Player` OtherActor))
      (`/Game/LHM/LHM_BP/Player/Blueprints/BP_LHM_Player.Damage` _asbp_lhm_player _damage))
    (:`then_1`
      (bind _asbp_enemy_base (cast `/Game/CHJ/Blueprints/BP_EnemyBase` OtherActor))
      (`/Game/CHJ/Blueprints/BP_EnemyFSM.Damage` (`self.GetComponentByClass` _asbp_enemy_base "/Game/CHJ/Blueprints/BP_EnemyFSM.BP_EnemyFSM_C") _damage))))

(event `self.CameraCollsion.OnComponentBeginOverlap`
  (params (OverlappedComponent :type "PrimitiveComponent Object Reference") (OtherActor :type "Actor Object Reference") (OtherComp :type "PrimitiveComponent Object Reference") (OtherBodyIndex :type Integer) (bFromSweep :type Boolean) (SweepResult :type "HitResult Structure (by ref)"))
  ;[1 1 1] Camera Shake
  (bind _asbp_lhm_player (cast `/Game/LHM/LHM_BP/Player/Blueprints/BP_LHM_Player` OtherActor))
  (bind _returnvalue (`self.K2_GetActorLocation` _asbp_lhm_player))
  (`GameplayStatics.PlayWorldCameraShake` "/Game/LDG/Blueprint/BP_ExplosionShake.BP_ExplosionShake_C" _returnvalue 100.0 1000.0)
  (`|SpawnActorFromClass` "/Game/LDG/Blueprint/BP_ProjectileField.BP_ProjectileField_C" (`KismetMathLibrary.MakeTransform` _returnvalue (struct) (3.0 3.0 3.0)) "Undefined" "MultiplyWithRoot" null null))

(fn `UserConstructionScript`)