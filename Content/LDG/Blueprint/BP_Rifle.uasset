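; BP_Rifle is the player's hitscan rifle, with a laser pointer that turns toward the player's TargetLocation every tick.
; Fire spends ammo, plays muzzle effects and multi-line traces from the muzzle to that target.
; Each hit spawns a BP_ProjectileField; enemy hits also subtract HP and add score on the game mode.
; Reload refills ammo after a delay, using stats held on BPGunComponent.
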(event `self.ReceiveBeginPlay`
  ;[1 1 1] Set Character
  (`parent.ReceiveBeginPlay`)
  (bind _returnvalue (`GameplayStatics.GetActorOfClass` "/Game/LHM/LHM_BP/Player/Blueprints/BP_LHM_Player.BP_LHM_Player_C"))
  (set `self.Character` _returnvalue))

(event `self.ReceiveTick`
  (params (DeltaSeconds :type "Float (single-precision)"))
  (bind _bp_laserpointcomp (`self.BP_LaserPointComp`))
  ;[1 1 1] Set LaserPointer Rotation
  (`parent.ReceiveTick` DeltaSeconds)
  (`SceneComponent.K2_SetWorldRotation` _bp_laserpointcomp (`KismetMathLibrary.FindLookAtRotation` (`SceneComponent.K2_GetComponentLocation` _bp_laserpointcomp) (`/Game/LHM/LHM_BP/Player/Blueprints/BP_LHM_Player.TargetLocation` (`self.Character`))) false false))

(event `/Game/LDG/Blueprint/BPI_Gun.Fire`
  (bind _bp_guncomponent (`self.BP_GunComponent`))
  (bind _returnvalue (`SceneComponent.GetSocketLocation` _bp_guncomponent "MuzzleFlash"))
  ;[1 1 1] Rifle Actions
  (set `/Game/LDG/Blueprint/BP_GunComponent.Ammo` (- (`/Game/LDG/Blueprint/BP_GunComponent.Ammo` _bp_guncomponent) 1) _bp_guncomponent)
  (`GameplayStatics.SpawnEmitterAtLocation` "/Game/Asset/MilitaryWeapSilver/FX/P_AssaultRifle_MuzzleFlash.P_AssaultRifle_MuzzleFlash" _returnvalue (struct) (0.5 0.5 0.5))
  (`GameplayStatics.PlaySound2D` "/Game/Asset/MilitaryWeapSilver/Sound/Rifle/Wavs/RifleA_Fire01.RifleA_Fire01" 1.0 1.0 0.0 null null)
  (bind _outhits (`KismetSystemLibrary.LineTraceMulti` _returnvalue (`/Game/LHM/LHM_BP/Player/Blueprints/BP_LHM_Player.TargetLocation` (`self.Character`)) "TraceTypeQuery1"))
  (for _array_element _outhits
    (`|ExecutionSequence`
      (:`then_0`
        (bind (_bblockinghit _binitialoverlap _time _distance _location _impactpoint _normal _impactnormal _physmat _hitactor) (`GameplayStatics.BreakHitResult` _array_element))
        ;[1 1 1] Damage
        (bind _asbp_enemy_base (cast `/Game/CHJ/Blueprints/BP_EnemyBase` _hitactor))
        (set `/Game/CHJ/Blueprints/BP_EnemyBase.CurrHp` (- (`/Game/CHJ/Blueprints/BP_EnemyBase.CurrHp` _asbp_enemy_base) (`/Game/LDG/Blueprint/BP_GunComponent.Damage` (`self.BP_GunComponent`))) _asbp_enemy_base)
        (bind _asbp_main_game_mode (cast `/Game/Main/BP_MainGameMode` (`GameplayStatics.GetGameMode`)))
        (set `/Game/Main/BP_MainGameMode.Score` (+ (`/Game/Main/BP_MainGameMode.Score` _asbp_main_game_mode) 1) _asbp_main_game_mode))
      (:`then_1`
        (`|SpawnActorFromClass` "/Game/LDG/Blueprint/BP_ProjectileField.BP_ProjectileField_C" (`KismetMathLibrary.MakeTransform` _location) "Undefined" "MultiplyWithRoot" null null)))))

(event `/Game/LDG/Blueprint/BPI_Gun.Reload`
  (bind _bp_guncomponent (`self.BP_GunComponent`))
  ;[1 1 1] Rifle Actions
  (`KismetSystemLibrary.PrintString` "Reloading...")
  (`KismetSystemLibrary.Delay` (`/Game/LDG/Blueprint/BP_GunComponent.ReloadTime` _bp_guncomponent))
  (set `/Game/LDG/Blueprint/BP_GunComponent.Ammo` (`/Game/LDG/Blueprint/BP_GunComponent.MaxAmmo` _bp_guncomponent) _bp_guncomponent)
  (`KismetSystemLibrary.PrintString` "Reloaded!"))

(fn `UserConstructionScript`
  (`parent.UserConstructionScript`))