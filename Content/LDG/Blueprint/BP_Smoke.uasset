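; BP_Smoke is a thrown smoke grenade that flags enemies caught in its cloud.
; MainAttack launches the physics mesh along the player camera's forward vector, then after a delay hides it, spawns a steam emitter and enables query collision on BlineArea.
; Overlapping BP_Enemy actors get InSmoke set on their BPEnemyFSM.
; When the cloud expires, only the last overlapped enemy has InSmoke cleared before the actor destroys itself.
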(event `self.ReceiveBeginPlay`
  (bind _asbp_lhm_player (cast `/Game/LHM/LHM_BP/Player/Blueprints/BP_LHM_Player` (`GameplayStatics.GetPlayerCharacter` 0)))
  (set `self.Character` _asbp_lhm_player)
  (bind _asbp_enemy (cast `/Game/CHJ/Blueprints/BP_Enemy` (`self.GetOwner`)))
  (set `self.Enemy` _asbp_enemy))

(event `/Game/LDG/Blueprint/BPI_MainAttackable.MainAttack`
  (bind _smokemesh (`self.SmokeMesh`))
  (bind _smokemesh_2 (`self.SmokeMesh`))
  ;[1 1 1] Generate Smoke
  (`PrimitiveComponent.SetSimulatePhysics` _smokemesh_2 true)
  (`PrimitiveComponent.SetPhysicsLinearVelocity` _smokemesh_2 (* (`SceneComponent.GetForwardVector` (`/Game/LHM/LHM_BP/Player/Blueprints/BP_LHM_Player.FirstPersonCamera` (`self.Character`))) (`self.Speed`)) false "None")
  (`KismetSystemLibrary.Delay` 2.0)
  (`SceneComponent.SetVisibility` _smokemesh false false)
  (`GameplayStatics.SpawnEmitterAtLocation` "/Game/LDG/FX/P_Steam_Lit.P_Steam_Lit" (`SceneComponent.K2_GetComponentLocation` _smokemesh) (struct) (3.0 3.0 3.0))
  (`PrimitiveComponent.SetCollisionEnabled` (`self.BlineArea`) "QueryOnly")
  (`PrimitiveComponent.SetSimulatePhysics` (`self.SmokeMesh`) false)
  (`KismetSystemLibrary.Delay` 10.0)
  (set `/Game/CHJ/Blueprints/BP_EnemyFSM.InSmoke` false (`/Game/CHJ/Blueprints/BP_Enemy.BP_EnemyFSM` (stale `self.BlineArea.OnComponentBeginOverlap` _asbp_enemy)))
  (`self.K2_DestroyActor`))

(event `self.BlineArea.OnComponentBeginOverlap`
  (params (OverlappedComponent :type "PrimitiveComponent Object Reference") (OtherActor :type "Actor Object Reference") (OtherComp :type "PrimitiveComponent Object Reference") (OtherBodyIndex :type Integer) (bFromSweep :type Boolean) (SweepResult :type "HitResult Structure (by ref)"))
  (bind _asbp_enemy (cast `/Game/CHJ/Blueprints/BP_Enemy` OtherActor))
  (set `/Game/CHJ/Blueprints/BP_EnemyFSM.InSmoke` true (`/Game/CHJ/Blueprints/BP_Enemy.BP_EnemyFSM` _asbp_enemy)))

(fn `UserConstructionScript`)