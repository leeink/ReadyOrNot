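; State machine component for the surrendering enemy, ticking idle, chase, attack, attack delay, return, death and surrender states.
; Idle detects the player by range, view-cone dot product and line trace, then chases via AI MoveTo within a leash, firing the level's first-found BP_Rifle.
; Surrender waits while the player is near, then reveals the child actor and reverts to Idle.
; ChangeState mirrors state to the AnimBP; patrol logic is unused.
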(event `self.ReceiveBeginPlay`
  ;[1 1 1] Enemy 총 셋팅
  (bind _returnvalue (`GameplayStatics.GetActorOfClass` "/Game/LDG/Blueprint/BP_Rifle.BP_Rifle_C"))
  (set `self.Rifle` _returnvalue)
  ;[1 1 1] 플레이어 클래스 셋팅
  (bind _returnvalue_2 (`GameplayStatics.GetActorOfClass` "/Game/LHM/LHM_BP/Player/Blueprints/BP_LHM_Player.BP_LHM_Player_C"))
  (set `self.Player` _returnvalue_2)
  ;[1 1 1] Enemy셋팅
  (bind _asbp_real_surrender_enemy (cast `/Game/CHJ/Blueprints/BP_Real_Surrender_Enemy` (`self.GetOwner`)))
  (set `self.Enemy` _asbp_real_surrender_enemy)
  ;[1 1 1] Enemy 애니메이션 셋팅
  (bind _asabp_real_surrender_enemy (cast `/Game/CHJ/Blueprints/ABP_Real_Surrender_Enemy` (`SkeletalMeshComponent.GetAnimInstance` (`Character.Mesh` (`self.Enemy`)))))
  (set `self.EnemyAnim` _asabp_real_surrender_enemy)
  ;[1 1 1] Ai Controller 셋팅
  (bind _asaicontroller (cast `AIController` (`Pawn.GetController` (`self.Enemy`))))
  (set `self.AiController` _asaicontroller)
  ;[1 1 1] 시야각을 cos(시야각) 으로 하자
  (set `self.View Angle` (`KismetMathLibrary.DegCos` (* (`self.View Angle`) 0.5)))
  ;[1 1 1] 처음 위치 셋팅
  (set `self.Origin Pos` (`Actor.K2_GetActorLocation` (`self.Enemy`)))
  (set `self.IsDeath` false)
  (set `self.Surrender_CurrAttackTime` 0.0)
  (set `self.IsSurrender` false))

(event `self.ReceiveTick`
  (params (DeltaSeconds :type "Float (single-precision)"))
  ;[1 1 1] 플레이어가 유효하다면
  (`/Engine/EditorBlueprintResources/StandardMacros.IsValid` (`self.Player`)
    (:`Is Valid`
      (`|ExecutionSequence`
        (:`then_0`
          ;[1 1 1] 현재 Enemy의 상태를 변환
          (switch `/Game/CHJ/Blueprints/BP_EnemyState` (`self.currState`)
            (:`NewEnumerator0`
              (`self.UpdateIdle`))
            (:`NewEnumerator1`
              (`self.UpdateTraceMove`))
            (:`NewEnumerator2`
              (`self.UpdateAttack`))
            (:`NewEnumerator4`
              (`self.UpdateDeath`))
            (:`NewEnumerator5`
              (`self.UpdateAttackDelay`))
            (:`NewEnumerator6`
              (`self.UpdateReturn`))
            (:`NewEnumerator10`
              (`self.UpdateSurrender`))))
        (:`then_1`
          (set `self.IsDeath` (<= (`/Game/CHJ/Blueprints/BP_EnemyBase.CurrHp` (`self.Enemy`)) 0.0)))))))

(fn `Can Trace`
  (returns (can :type Boolean))
  (locals (dir :type "Vector Structure"))
  (bind _output_get (set `local.dir` (- (`Actor.K2_GetActorLocation` (`self.Player`)) (`Actor.K2_GetActorLocation` (`self.Enemy`)))))
  (if (< (`KismetMathLibrary.VSize` _output_get) (`self.Trace Range`))
    (if (> (`KismetMathLibrary.Dot_VectorVector` (`KismetMathLibrary.Normal` (`local.dir`)) (`Actor.GetActorForwardVector` (`self.Enemy`))) (`self.View Angle`))
      ;[1 1 1] 라인트레이스 실행 : 내 위치부터 ~ 플레이어 위치까지
      (bind (_outhit _returnvalue) (`KismetSystemLibrary.LineTraceSingle` :`Start` (`Actor.K2_GetActorLocation` (`self.Enemy`)) :`End` (`Actor.K2_GetActorLocation` (`self.Player`)) :`TraceChannel` "TraceTypeQuery1" :`DrawDebugType` "ForDuration"))
      ;[1 1 1] 플레이어가 탐색 되었다면 True
      (if _returnvalue
        (return (`KismetStringLibrary.Contains` (`KismetSystemLibrary.GetDisplayName` (`.HitActor` (`GameplayStatics.BreakHitResult` _outhit))) "Player")))
      (else
        (return false)))
    (else
      (return false))))

(fn `Change State`
  (params (State :type "/Game/CHJ/Blueprints/BP_EnemyState Enum" :default "NewEnumerator0"))
  (`KismetSystemLibrary.PrintString` (`KismetStringLibrary.Concat_StrStr` (`|GetEnumeratorNameAsString` (`self.currState`)) "---------->" (`|GetEnumeratorNameAsString` State)))
  (`Controller.StopMovement` (`self.AiController`))
  (bind _output_get (set `self.currState` (`local.state`)))
  (bind _output_get_2 (set `/Game/CHJ/Blueprints/ABP_Real_Surrender_Enemy.State` _output_get (`self.EnemyAnim`)))
  (set `self.currTime` 0.0)
  (switch `/Game/CHJ/Blueprints/BP_EnemyState` _output_get_2))

(fn `IsWaitComplete`
  (params (delay :type "Float (double-precision)"))
  (returns (complete :type Boolean))
  (bind _output_get (set `self.currTime` (+ (`self.currTime`) (`GameplayStatics.GetWorldDeltaSeconds`))))
  (return (> _output_get (`local.delay`))))

(fn `UpdateAttack`
  (if (`self.IsDeath`)
    (`self.Change State` "NewEnumerator4")
    (else
      ;[1 1 1] 공격할 때마다, 플레이어 방향으로
      (`Actor.K2_SetActorRotation` (`self.Enemy`) (`KismetMathLibrary.Conv_VectorToRotator` (`KismetMathLibrary.Normal` (- (`Actor.K2_GetActorLocation` (`self.Player`)) (`Actor.K2_GetActorLocation` (`self.Enemy`))))) false)
      (message `/Game/LDG/Blueprint/BPI_Gun.Fire` (`self.Rifle`))
      (`self.Change State` "NewEnumerator5"))))

(fn `UpdateAttackDelay`
  (if (`self.IsDeath`)
    (`self.Change State` "NewEnumerator4")
    (else
      (bind _output_get (set `self.currTime` (+ (`self.currTime`) (`GameplayStatics.GetWorldDeltaSeconds`))))
      ;[1 1 1] Max 시간을 넘었으면 초기화
      (if (> _output_get (`self.attackDelayTime`))
        (set `self.currTime` 0.0)
        ;[1 1 1] 만약에 Attack Range 플레이어가 있다면 공격
        (if (< (`KismetMathLibrary.Vector_Distance` (`Actor.K2_GetActorLocation` (`self.Player`)) (`Actor.K2_GetActorLocation` (`self.Enemy`))) (`self.AttackRange`))
          (`self.Change State` "NewEnumerator2")
          (else
            (bind _can (`self.Can Trace`))
            (if _can
              (`self.Change State` "NewEnumerator1")
              (else
                (`self.Change State` "NewEnumerator0")))))))))

(fn `UpdateDeath`
  (`PrimitiveComponent.SetCollisionProfileName` (`Character.Mesh` (`self.Enemy`)) "Ragdoll" true)
  (`PrimitiveComponent.SetSimulatePhysics` (`Character.Mesh` (`self.Enemy`)) true)
  (`PrimitiveComponent.SetCollisionEnabled` (`Character.CapsuleComponent` (`self.Enemy`)) "NoCollision"))

(fn `UpdateIdle`
  (if (`self.IsDeath`)
    (`self.Change State` "NewEnumerator4")
    (else
      ;[1 1 1] 플레이어를 탐색 했나? 탐색했다면 움직여라 / 못했다면 순찰해라
      (bind _can (`self.Can Trace`))
      (if _can
        (`self.Change State` "NewEnumerator1")
        (else
          ;[1 1 1] 딜레이
          (`self.IsWaitComplete` 2.0))))))

(fn `UpdatePatrolMove`
  (if (`self.IsDeath`)
    (`self.Change State` "NewEnumerator4")
    (elif (< (`KismetMathLibrary.Vector_Distance` (`Actor.K2_GetActorLocation` (`self.Enemy`)) (`self.PatrolPos`)) 50.0)
      (`self.Change State` "NewEnumerator0")
      (else
        (bind _can (`self.Can Trace`))
        (if _can
          (`self.Change State` "NewEnumerator2"))))))

(fn `UpdateReturn`
  (bind _returnvalue (`AIController.MoveToLocation` (`self.AiController`) (`self.Origin Pos`) -1.0 true true false true null true))
  (if (`|EnumEquality` _returnvalue "AlreadyAtGoal")
    (`self.Change State` "NewEnumerator0")))

(fn `UpdateSurrender`
  (if (`self.IsDeath`)
    (`self.Change State` "NewEnumerator4")
    (elif (>= (`self.SurrenderRange`) (`KismetMathLibrary.Vector_Distance` (`Actor.K2_GetActorLocation` (`self.Enemy`)) (`Actor.K2_GetActorLocation` (`self.Player`))))
      (bind _output_get (set `self.Surrender_CurrAttackTime` (+ (`self.Surrender_CurrAttackTime`) (`GameplayStatics.GetWorldDeltaSeconds`))))
      (if (>= _output_get (`self.Surrender_MaxAttackTime`))
        (set `self.IsSurrender` true)
        (bind _complete (`self.IsWaitComplete` 1.0))
        (if _complete
          (`SceneComponent.SetVisibility` (`/Game/CHJ/Blueprints/BP_Real_Surrender_Enemy.ChildActor` (`self.Enemy`)) true false)
          (bind _complete_2 (`self.IsWaitComplete` 3.0))
          (if _complete_2
            (`self.Change State` "NewEnumerator0")))))))

(fn `UpdateTraceMove`
  (locals (dir :type "Vector Structure") (dist :type "Float (double-precision)"))
  (if (`self.IsDeath`)
    (`self.Change State` "NewEnumerator4")
    (elif (> (`KismetMathLibrary.Vector_Distance` (`self.Origin Pos`) (`Actor.K2_GetActorLocation` (`self.Enemy`))) (`self.MoveRange`))
      ;[1 1 1] 원래 자리로 되돌아가기
      (`self.Change State` "NewEnumerator6")
      (else
        (bind _output_get (set `local.dir` (- (`Actor.K2_GetActorLocation` (`self.Player`)) (`Actor.K2_GetActorLocation` (`self.Enemy`)))))
        (set `local.dist` (`KismetMathLibrary.VSize` _output_get))
        ;[1 1 1] AI Navigation
        (`AIController.MoveToLocation` (`self.AiController`) (`Actor.K2_GetActorLocation` (`self.Player`)) -1.0 true true false true null true)
        ;[1 1 1] 만약에 플레이어가 Attack Range 에 들어왔다면 ATTACK 상태로 바꿔라
        (if (< (`local.dist`) (`self.AttackRange`))
          (`self.Change State` "NewEnumerator2"))))))